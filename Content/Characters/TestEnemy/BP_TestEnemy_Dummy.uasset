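; Test dummy enemy character that shows a health bar and applies regeneration and immortality effects to itself.
; On BeginPlay it creates a healthbar widget for its widget component and binds the widget's HealthViewModel to its Deck ability system component.
; It then applies the regen and immortal Gameplay Effects through its Ability System Component.
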(event EventBeginPlay
  (Utilities|FlowControl|Sequence
    (:then_0
      (bind _returnvalue (UserInterface|CreateWidget "/Game/UI/HUD/Healthbar/WBP_Healthbar.WBP_Healthbar_C"))
      (UserInterface|SetWidget (Variables|Default|GetHealthbarWidget) _returnvalue)
      (bind _asdeck_ability_system_component (Utilities|Casting|CastToDeckAbilitySystemComponent (Ability|GetAbilitySystemComponent 0)))
      (Class|HealthViewModel|BindAttributeSet (Variables|/Game/UI/HUD/Healthbar/WBP_Healthbar.WBP_Healthbar_C|GetHealthViewModel _returnvalue) _asdeck_ability_system_component))
    (:then_1
      (bind _returnvalue_2 (Spec|MakeSpecHandle(ByClass) "/Game/Abilities/Effects/GE_Regen.GE_Regen_C" 0))
      (GameplayEffects|ApplyGameplayEffectSpecToSelf (Variables|Default|GetAbilitySystemComponent) _returnvalue_2)
      (bind _returnvalue_3 (Spec|MakeSpecHandle(ByClass) "/Game/Abilities/Effects/GE_Immortal.GE_Immortal_C" 0))
      (GameplayEffects|ApplyGameplayEffectSpecToSelf (Variables|Default|GetAbilitySystemComponent) _returnvalue_3))))

(fn ConstructionScript)